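; Base character Blueprint that animates VR hand meshes and, without an HMD, shows the player's net role on an overhead widget.
; With an HMD, BeginPlay mirrors the left hand's ABP_MannequinsXR instance.
; Enhanced Input drives each hand's pose alphas: grasp and index curl follow action values, while point and thumb-up switch inversely, zero on start and one on completion.
; Slide and roll montage sequences with capsule shrinking are unconnected and never run.
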(event Input|EnhancedActionEvents|EnhancedInputActionIA_Hand_Grasp_Left
  (params (ActionValue :type Float%20%28double-precision%29) (ElapsedSeconds :type Float%20%28double-precision%29) (TriggeredSeconds :type Float%20%28double-precision%29) (InputAction :type Input%20Action%20Object%20Reference :default "/Game/VRTemplate/Input/Actions/Hands/IA_Hand_Grasp_Left.IA_Hand_Grasp_Left"))
  (bind _lefthandmesh (Variables|Default|GetLeftHandMesh))
  (bind _returnvalue (Components|SkeletalMesh|GetAnimInstance _lefthandmesh))
  (:Triggered
    (bind _asabp_mannequins_xr (Utilities|Casting|CastToABP_MannequinsXR _returnvalue))
    (Variables|/Game/Characters/MannequinsXR/Meshes/ABP_MannequinsXR.ABP_MannequinsXR_C|SetPoseAlphaGrasp _asabp_mannequins_xr ActionValue))
  (:Canceled
    (bind _asabp_mannequins_xr_2 (Utilities|Casting|CastToABP_MannequinsXR _returnvalue :!label _label))
    (Variables|/Game/Characters/MannequinsXR/Meshes/ABP_MannequinsXR.ABP_MannequinsXR_C|SetPoseAlphaGrasp _asabp_mannequins_xr_2 0.0))
  (:Completed
    (goto _label)))

(event Input|EnhancedActionEvents|EnhancedInputActionIA_Hand_Point_Left
  (params (ActionValue :type Float%20%28double-precision%29) (ElapsedSeconds :type Float%20%28double-precision%29) (TriggeredSeconds :type Float%20%28double-precision%29) (InputAction :type Input%20Action%20Object%20Reference :default "/Game/VRTemplate/Input/Actions/Hands/IA_Hand_Point_Left.IA_Hand_Point_Left"))
  (bind _lefthandmesh (Variables|Default|GetLeftHandMesh))
  (:Started
    (bind _asabp_mannequins_xr (Utilities|Casting|CastToABP_MannequinsXR (Components|SkeletalMesh|GetAnimInstance _lefthandmesh) :!label _label))
    (Variables|/Game/Characters/MannequinsXR/Meshes/ABP_MannequinsXR.ABP_MannequinsXR_C|SetPoseAlphaPoint _asabp_mannequins_xr 0.0))
  (:Canceled
    (goto _label))
  (:Completed
    (bind _asabp_mannequins_xr_2 (Utilities|Casting|CastToABP_MannequinsXR (Components|SkeletalMesh|GetAnimInstance _lefthandmesh)))
    (Variables|/Game/Characters/MannequinsXR/Meshes/ABP_MannequinsXR.ABP_MannequinsXR_C|SetPoseAlphaPoint _asabp_mannequins_xr_2 1.0)))

(event Input|EnhancedActionEvents|EnhancedInputActionIA_Hand_ThumbUp_Left
  (params (ActionValue :type Float%20%28double-precision%29) (ElapsedSeconds :type Float%20%28double-precision%29) (TriggeredSeconds :type Float%20%28double-precision%29) (InputAction :type Input%20Action%20Object%20Reference :default "/Game/VRTemplate/Input/Actions/Hands/IA_Hand_ThumbUp_Left.IA_Hand_ThumbUp_Left"))
  (bind _lefthandmesh (Variables|Default|GetLeftHandMesh))
  (:Started
    (bind _asabp_mannequins_xr (Utilities|Casting|CastToABP_MannequinsXR (Components|SkeletalMesh|GetAnimInstance _lefthandmesh) :!label _label))
    (Variables|/Game/Characters/MannequinsXR/Meshes/ABP_MannequinsXR.ABP_MannequinsXR_C|SetPoseAlphaThumbUp _asabp_mannequins_xr 0.0))
  (:Canceled
    (goto _label))
  (:Completed
    (bind _asabp_mannequins_xr_2 (Utilities|Casting|CastToABP_MannequinsXR (Components|SkeletalMesh|GetAnimInstance _lefthandmesh)))
    (Variables|/Game/Characters/MannequinsXR/Meshes/ABP_MannequinsXR.ABP_MannequinsXR_C|SetPoseAlphaThumbUp _asabp_mannequins_xr_2 1.0)))

(event Input|EnhancedActionEvents|EnhancedInputActionIA_Hand_IndexCurl_Right
  (params (ActionValue :type Float%20%28double-precision%29) (ElapsedSeconds :type Float%20%28double-precision%29) (TriggeredSeconds :type Float%20%28double-precision%29) (InputAction :type Input%20Action%20Object%20Reference :default "/Game/VRTemplate/Input/Actions/Hands/IA_Hand_IndexCurl_Right.IA_Hand_IndexCurl_Right"))
  (bind _righthandmesh (Variables|Default|GetRightHandMesh))
  (bind _returnvalue (Components|SkeletalMesh|GetAnimInstance _righthandmesh))
  (:Triggered
    (bind _asabp_mannequins_xr (Utilities|Casting|CastToABP_MannequinsXR _returnvalue))
    (Variables|/Game/Characters/MannequinsXR/Meshes/ABP_MannequinsXR.ABP_MannequinsXR_C|SetPoseAlphaIndexCurl _asabp_mannequins_xr ActionValue))
  (:Canceled
    (bind _asabp_mannequins_xr_2 (Utilities|Casting|CastToABP_MannequinsXR _returnvalue :!label _label))
    (Variables|/Game/Characters/MannequinsXR/Meshes/ABP_MannequinsXR.ABP_MannequinsXR_C|SetPoseAlphaIndexCurl _asabp_mannequins_xr_2 0.0))
  (:Completed
    (goto _label)))

(event Input|EnhancedActionEvents|EnhancedInputActionIA_Hand_Grasp_Right
  (params (ActionValue :type Float%20%28double-precision%29) (ElapsedSeconds :type Float%20%28double-precision%29) (TriggeredSeconds :type Float%20%28double-precision%29) (InputAction :type Input%20Action%20Object%20Reference :default "/Game/VRTemplate/Input/Actions/Hands/IA_Hand_Grasp_Right.IA_Hand_Grasp_Right"))
  (bind _righthandmesh (Variables|Default|GetRightHandMesh))
  (bind _returnvalue (Components|SkeletalMesh|GetAnimInstance _righthandmesh))
  (:Triggered
    (bind _asabp_mannequins_xr (Utilities|Casting|CastToABP_MannequinsXR _returnvalue))
    (Variables|/Game/Characters/MannequinsXR/Meshes/ABP_MannequinsXR.ABP_MannequinsXR_C|SetPoseAlphaGrasp _asabp_mannequins_xr ActionValue))
  (:Canceled
    (bind _asabp_mannequins_xr_2 (Utilities|Casting|CastToABP_MannequinsXR _returnvalue :!label _label))
    (Variables|/Game/Characters/MannequinsXR/Meshes/ABP_MannequinsXR.ABP_MannequinsXR_C|SetPoseAlphaGrasp _asabp_mannequins_xr_2 0.0))
  (:Completed
    (goto _label)))

(event Input|EnhancedActionEvents|EnhancedInputActionIA_Hand_IndexCurl_Left
  (params (ActionValue :type Float%20%28double-precision%29) (ElapsedSeconds :type Float%20%28double-precision%29) (TriggeredSeconds :type Float%20%28double-precision%29) (InputAction :type Input%20Action%20Object%20Reference :default "/Game/VRTemplate/Input/Actions/Hands/IA_Hand_IndexCurl_Left.IA_Hand_IndexCurl_Left"))
  (bind _lefthandmesh (Variables|Default|GetLeftHandMesh))
  (bind _returnvalue (Components|SkeletalMesh|GetAnimInstance _lefthandmesh))
  (:Triggered
    (bind _asabp_mannequins_xr (Utilities|Casting|CastToABP_MannequinsXR _returnvalue))
    (Variables|/Game/Characters/MannequinsXR/Meshes/ABP_MannequinsXR.ABP_MannequinsXR_C|SetPoseAlphaIndexCurl _asabp_mannequins_xr ActionValue))
  (:Canceled
    (bind _asabp_mannequins_xr_2 (Utilities|Casting|CastToABP_MannequinsXR _returnvalue :!label _label))
    (Variables|/Game/Characters/MannequinsXR/Meshes/ABP_MannequinsXR.ABP_MannequinsXR_C|SetPoseAlphaIndexCurl _asabp_mannequins_xr_2 0.0))
  (:Completed
    (goto _label)))

(event Input|EnhancedActionEvents|EnhancedInputActionIA_Hand_ThumbUp_Right
  (params (ActionValue :type Float%20%28double-precision%29) (ElapsedSeconds :type Float%20%28double-precision%29) (TriggeredSeconds :type Float%20%28double-precision%29) (InputAction :type Input%20Action%20Object%20Reference :default "/Game/VRTemplate/Input/Actions/Hands/IA_Hand_ThumbUp_Right.IA_Hand_ThumbUp_Right"))
  (bind _righthandmesh (Variables|Default|GetRightHandMesh))
  (:Started
    (bind _asabp_mannequins_xr (Utilities|Casting|CastToABP_MannequinsXR (Components|SkeletalMesh|GetAnimInstance _righthandmesh) :!label _label))
    (Variables|/Game/Characters/MannequinsXR/Meshes/ABP_MannequinsXR.ABP_MannequinsXR_C|SetPoseAlphaThumbUp _asabp_mannequins_xr 0.0))
  (:Canceled
    (goto _label))
  (:Completed
    (bind _asabp_mannequins_xr_2 (Utilities|Casting|CastToABP_MannequinsXR (Components|SkeletalMesh|GetAnimInstance _righthandmesh)))
    (Variables|/Game/Characters/MannequinsXR/Meshes/ABP_MannequinsXR.ABP_MannequinsXR_C|SetPoseAlphaThumbUp _asabp_mannequins_xr_2 1.0)))

(event Input|EnhancedActionEvents|EnhancedInputActionIA_Hand_Point_Right
  (params (ActionValue :type Float%20%28double-precision%29) (ElapsedSeconds :type Float%20%28double-precision%29) (TriggeredSeconds :type Float%20%28double-precision%29) (InputAction :type Input%20Action%20Object%20Reference :default "/Game/VRTemplate/Input/Actions/Hands/IA_Hand_Point_Right.IA_Hand_Point_Right"))
  (bind _righthandmesh (Variables|Default|GetRightHandMesh))
  (:Started
    (bind _asabp_mannequins_xr (Utilities|Casting|CastToABP_MannequinsXR (Components|SkeletalMesh|GetAnimInstance _righthandmesh) :!label _label))
    (Variables|/Game/Characters/MannequinsXR/Meshes/ABP_MannequinsXR.ABP_MannequinsXR_C|SetPoseAlphaPoint _asabp_mannequins_xr 0.0))
  (:Canceled
    (goto _label))
  (:Completed
    (bind _asabp_mannequins_xr_2 (Utilities|Casting|CastToABP_MannequinsXR (Components|SkeletalMesh|GetAnimInstance _righthandmesh)))
    (Variables|/Game/Characters/MannequinsXR/Meshes/ABP_MannequinsXR.ABP_MannequinsXR_C|SetPoseAlphaPoint _asabp_mannequins_xr_2 1.0)))

(event EventBeginPlay
  (if (Class|HeadMountedDisplayFunctionLibrary|IsHeadMountedDisplayEnabled)
    (bind _asabp_mannequins_xr (Utilities|Casting|CastToABP_MannequinsXR (Components|SkeletalMesh|GetAnimInstance (Variables|Default|GetLeftHandMesh))))
    (Variables|/Game/Characters/MannequinsXR/Meshes/ABP_MannequinsXR.ABP_MannequinsXR_C|SetbMirror _asabp_mannequins_xr true)
    (else
      (bind _aswbp_overhead_widget (Utilities|Casting|CastToWBP_OverheadWidget (UserInterface|GetUserWidgetObject (Variables|Default|GetOverheadWidget))))
      (Class|OverheadWidget|ShowPlayerNetRole _aswbp_overhead_widget self))))

(event Collision|EventActorBeginOverlap
  (params (OtherActor :type Actor%20Object%20Reference)))

(event EventTick
  (params (DeltaSeconds :type Float%20%28single-precision%29)))

(event Input|ActionEvents|InputActionRolling
  (params (Key :type Key%20Structure :default "None")))

(event Input|ActionEvents|InputActionSliding
  (params (Key :type Key%20Structure :default "None")))

(fn ConstructionScript)