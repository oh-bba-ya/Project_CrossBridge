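; BP_Test_Gun is a test gun actor that automatically fires a repeating volley of three bullet types with no input.
; Tick drives a chain of latent Delays, which ignore re-triggers while pending and so act as a repeating timer.
; After each longer wait it spawns a base bullet, then ice and lightning variants at short intervals, all at the SpawnArrow transform.
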(event EventBeginPlay)

(event Collision|EventActorBeginOverlap
  (params (OtherActor :type Actor%20Object%20Reference)))

(event EventTick
  (params (DeltaSeconds :type Float%20%28single-precision%29))
  (Utilities|FlowControl|Delay 3.0)
  (Game|SpawnActorfromClass "/Game/HYY/BluePrint/BP_Test_Bullet.BP_Test_Bullet_C" (Transformation|GetWorldTransform (Variables|Default|GetSpawn%20Arrow)) "Undefined" 0 0)
  (Utilities|FlowControl|Delay 0.5)
  (Game|SpawnActorfromClass "/Game/HYY/BluePrint/BP_Test_Bullet_ice.BP_Test_Bullet_ice_C" (Transformation|GetWorldTransform (Variables|Default|GetSpawn%20Arrow)) "Undefined" 0 0)
  (Utilities|FlowControl|Delay 0.5)
  (Game|SpawnActorfromClass "/Game/HYY/BluePrint/BP_Test_Bullet_lightning.BP_Test_Bullet_lightning_C" (Transformation|GetWorldTransform (Variables|Default|GetSpawn%20Arrow)) "Undefined" 0 0))

(fn ConstructionScript)